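; BP_NPC is a talkable NPC that shows its dialogue lines one at a time on the player's HUD.
; Its TalkingZone overlap registers it as the third-person character's CurrentNPC, and leaving clears that reference, the text and the dialogue index.
; IncrementDialogue, not called within this Blueprint, displays the current Dialogue entry and advances the index, resetting it and blanking the text when it overruns the array.
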(event `self.TalkingZone.OnComponentBeginOverlap`
  (params (OverlappedComponent :type "PrimitiveComponent Object Reference") (OtherActor :type "Actor Object Reference") (OtherComp :type "PrimitiveComponent Object Reference") (OtherBodyIndex :type Integer) (bFromSweep :type Boolean) (SweepResult :type "HitResult Structure (by ref)"))
  (bind _asbp_third_person_character (cast `/Game/ThirdPerson/Blueprints/BP_ThirdPersonCharacter` OtherActor))
  (set `/Game/ThirdPerson/Blueprints/BP_ThirdPersonCharacter.CurrentNPC` self _asbp_third_person_character))

(event `self.TalkingZone.OnComponentEndOverlap`
  (params (OverlappedComponent :type "PrimitiveComponent Object Reference") (OtherActor :type "Actor Object Reference") (OtherComp :type "PrimitiveComponent Object Reference") (OtherBodyIndex :type Integer))
  (bind _asbp_third_person_character (cast `/Game/ThirdPerson/Blueprints/BP_ThirdPersonCharacter` OtherActor))
  (set `/Game/ThirdPerson/Blueprints/BP_ThirdPersonCharacter.CurrentNPC` null _asbp_third_person_character)
  (`TextBlock.SetText` (`/Game/WBP_HUD.Txt_Dialogue` (`/Game/ThirdPerson/Blueprints/BP_ThirdPersonCharacter.HUD` _asbp_third_person_character)) "")
  (set `self.DialogueIndex` 0))

(fn `IncrementDialogue`
  (params (PlayerRef :type "/Game/ThirdPerson/Blueprints/BP_ThirdPersonCharacter Object Reference"))
  ;[1 1 1] Set text to be whichever element of dialogue we are at
  (`TextBlock.SetText` (`/Game/WBP_HUD.Txt_Dialogue` (`/Game/ThirdPerson/Blueprints/BP_ThirdPersonCharacter.HUD` PlayerRef)) (`|GetArrayItem` (`self.Dialogue`) (`self.DialogueIndex`)))
  ;[1 1 1] Increment Dialogue Index
  (bind _result (`/Engine/EditorBlueprintResources/StandardMacros.IncrementInt` (`self.DialogueIndex`))
    (:`  `
      ;[1 1 1] If we've run out of dialogue, reset dialogue index
      (if (> _result (`KismetArrayLibrary.Array_Length` (`self.Dialogue`)))
        (set `self.DialogueIndex` 0)
        ;[1 1 1] Clear dialogue on screen
        (`TextBlock.SetText` (`/Game/WBP_HUD.Txt_Dialogue` (`/Game/ThirdPerson/Blueprints/BP_ThirdPersonCharacter.HUD` (`local.PlayerRef`))) "")))))

(fn `UserConstructionScript`)